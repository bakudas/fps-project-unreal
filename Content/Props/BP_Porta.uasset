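; BP_Porta is an interactive door that can be locked to a colored key, tinted yellow or red through a dynamic material at BeginPlay.
; Box overlap stores the BP_Personagem reference used for key checks.
; Interaction requires a key matching CorChave when locked, printing a message otherwise.
; A FlipFlop alternates playing and reversing a timeline that drives the door's yaw to open and close it.
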(event `self.ReceiveBeginPlay`
  (`|ExecutionSequence`
    (:`then_0`
      (bind _returnvalue (`PrimitiveComponent.CreateDynamicMaterialInstance` (`self.Cube`) 0 null "None"))
      (bind _output_get (set `self.MaterialDoor` _returnvalue)))
    (:`then_1`
      (switch `string` (`self.CorChave`)
        (:`Amarelo`
          (bind _output_get_2 (set `self.ColorDoor` (struct :`R` 0.885417 :`G` 0.563084 :`A` 1.0)))
          (`MaterialInstanceDynamic.SetVectorParameterValue` _output_get "CorBase" _output_get_2))
        (:`Vermelho`
          (bind _output_get_3 (set `self.ColorDoor` (struct :`R` 1.0 :`G` 0.008924 :`A` 1.0)))
          (`MaterialInstanceDynamic.SetVectorParameterValue` _output_get "CorBase" _output_get_3))))))

(event `/Game/Game/BP_Interface.Interaction`
  (bind _personagem (`self.Personagem`))
  ;[1 1 1] Abrir / Fechar Porta
  (if (`self.IsLocked`)
    (if (`/Game/Personagem/BP_Personagem.HasKey` _personagem)
      (if (`BlueprintSetLibrary.Set_Contains` (`/Game/Personagem/BP_Personagem.KeyColor` _personagem) (`self.CorChave`))
        (`/Engine/EditorBlueprintResources/StandardMacros.FlipFlop` :!label _label
          (:`A`
            (bind (_direction `_rotação`) (`Timeline|Abrir / Fechar Porta` :!via `PlayFromStart` :!label _label_2)
              (:`Update`
                (`SceneComponent.K2_SetRelativeRotation` (`self.porta`) (`KismetMathLibrary.MakeRotator` 0.0 0.0 `_rotação`) false false))))
          (:`B`
            (goto _label_2 :!via `ReverseFromEnd`)))
        (else
          (`KismetSystemLibrary.PrintString` "NAO TENHO CHAVE" :!label _label_3)))
      (else
        (goto _label_3)))
    (else
      (goto _label))))

(event `self.Box.OnComponentBeginOverlap`
  (params (OverlappedComponent :type "PrimitiveComponent Object Reference") (OtherActor :type "Actor Object Reference") (OtherComp :type "PrimitiveComponent Object Reference") (OtherBodyIndex :type Integer) (bFromSweep :type Boolean) (SweepResult :type "HitResult Structure (by ref)"))
  (bind _output_get (set `self.Hit Actor` OtherActor))
  (bind _asbp_personagem (cast `/Game/Personagem/BP_Personagem` _output_get))
  (bind _output_get_2 (set `self.Personagem` _asbp_personagem))
  (`KismetSystemLibrary.PrintString` (`KismetSystemLibrary.GetDisplayName` _output_get_2)))

(fn `PlayerHasKeys`)

(fn `UserConstructionScript`)