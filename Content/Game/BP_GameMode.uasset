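; Game mode that holds score, player health (Vida) and ammo (Munição) and offers functions to change them.
; AddScore assigns the passed value rather than accumulating it, then calls PrintScore; BeginPlay uses it to set a starting score.
; DanoJogador, CuraJogador and AddMunição apply unclamped damage, healing and ammo gains, printing the result.
; CuraJogador's printout adds the heal amount again, so it differs from the stored health.
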(event `self.ReceiveBeginPlay`
  (`self.AddScore` 2500))

(event `self.ReceiveTick`
  (params (DeltaSeconds :type "Float (single-precision)")))

(fn `AddMunição`
  (params (`QtdMunição` :type Integer))
  (bind _output_get (set `self.Munição` (+ `QtdMunição` (`self.Munição`))))
  (`KismetSystemLibrary.PrintString` (`KismetStringLibrary.Conv_IntToString` _output_get)))

(fn `AddScore`
  (params (Score :type Integer))
  (set `self.Score` Score)
  (`self.PrintScore`))

(fn `CuraJogador`
  (params (CuraAmount :type Integer))
  (bind _returnvalue (+ (`self.Vida`) CuraAmount))
  (set `self.Vida` _returnvalue)
  (`KismetSystemLibrary.PrintString` (`KismetStringLibrary.Conv_IntToString` _returnvalue)))

(fn `DanoJogador`
  (params (Dano :type Integer))
  (bind _output_get (set `self.Vida` (- (`self.Vida`) Dano)))
  (`KismetSystemLibrary.PrintString` (`KismetStringLibrary.Conv_IntToString` _output_get)))

(fn `PrintScore`
  (`KismetSystemLibrary.PrintString` (`KismetStringLibrary.Conv_IntToString` (`self.Score`))))

(fn `UserConstructionScript`)