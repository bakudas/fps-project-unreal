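; BP_Arma_Child_Nerf is a child Blueprint for a Nerf gun pickup that arms whoever touches it.
; Tick spins its Pivot as a rotation effect.
; Any overlap with the Collider plays a pickup sound and particle burst, sends PlayerIsArmedMessage to the other actor without filtering, then destroys the pickup.
; The Interaction and PlayerHasKeys functions only return empty or false defaults.
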(event `self.ReceiveTick`
  (params (DeltaSeconds :type "Float (single-precision)"))
  ;[1 1 1] Rotation FX
  (`SceneComponent.K2_AddLocalRotation` (`self.pivot`) (`self.Rotation`) false false))

(event `self.Collider.OnComponentBeginOverlap`
  (params (OverlappedComponent :type "PrimitiveComponent Object Reference") (OtherActor :type "Actor Object Reference") (OtherComp :type "PrimitiveComponent Object Reference") (OtherBodyIndex :type Integer) (bFromSweep :type Boolean) (SweepResult :type "HitResult Structure (by ref)"))
  (bind _returnvalue (`self.K2_GetActorLocation`))
  ;[1 1 1] Pick Gun
  (`GameplayStatics.PlaySoundAtLocation` "/Engine/VREditor/Sounds/UI/Object_PickUp.Object_PickUp" _returnvalue (struct) 0.5 1.0 0.0 null null null)
  (`GameplayStatics.SpawnEmitterAtLocation` "/Game/Particulas/P_Item_Pickup.P_Item_Pickup" _returnvalue)
  (message `/Game/Game/BP_Interface.PlayerIsArmed` OtherActor)
  (`self.K2_DestroyActor`))

(fn `Interaction`
  (returns (Response :type String))
  (return ""))

(fn `PlayerHasKeys`
  (returns (HasKey :type Boolean))
  (return false))

(fn `UserConstructionScript`
  (`parent.UserConstructionScript`))