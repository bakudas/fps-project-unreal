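; BP_Coletavel_Child_Explosive is a child collectible Blueprint that damages the player as an explosive.
; Its Hit function prints a debug explosion message, then calls DanoJogador on BP_GameMode with the QtdDano amount.
; The Destroyed event repeats the same logic with a hard-coded damage value instead of the variable, so destruction from any cause also hurts the player.
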(event `self.ReceiveDestroyed`
  ;[1 1 1] Dano no Jogador
  (`KismetSystemLibrary.PrintString` "CACETE EXPLODIU")
  (bind _asbp_game_mode (cast `/Game/Game/BP_GameMode` (`GameplayStatics.GetGameMode`)))
  (`/Game/Game/BP_GameMode.DanoJogador` _asbp_game_mode 10))

(fn `Hit`
  ;[1 1 1] Dano no Jogador
  (`KismetSystemLibrary.PrintString` "CACETE EXPLODIU")
  (bind _asbp_game_mode (cast `/Game/Game/BP_GameMode` (`GameplayStatics.GetGameMode`)))
  (`/Game/Game/BP_GameMode.DanoJogador` _asbp_game_mode (`self.Qtd Dano`)))

(fn `UserConstructionScript`
  (`parent.UserConstructionScript`))