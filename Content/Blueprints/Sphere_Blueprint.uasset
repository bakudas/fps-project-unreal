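; Sphere actor that rotates in place and explodes when it hits something, damaging the player.
; Tick applies a local rotation, while Hit plays an explosion sound and particle effect at the impact point, then destroys the actor.
; The Destroyed event prints a debug message and calls DanoJogador on BP_GameMode, so player damage follows any destruction of the sphere, whatever its cause.
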(event `self.ReceiveTick`
  (params (DeltaSeconds :type "Float (single-precision)"))
  (`self.K2_AddActorLocalRotation` (`self.Delta Rotation`)))

(event `self.ReceiveHit`
  (params (MyComp :type "PrimitiveComponent Object Reference") (Other :type "Actor Object Reference") (OtherComp :type "PrimitiveComponent Object Reference") (bSelfMoved :type Boolean) (HitLocation :type "Vector Structure") (HitNormal :type "Vector Structure") (NormalImpulse :type "Vector Structure") (Hit :type "HitResult Structure (by ref)"))
  ;[1 1 1] Destroy
  (`GameplayStatics.PlaySoundAtLocation` "/Game/StarterContent/Audio/Explosion01.Explosion01" HitLocation (struct) 0.2 1.0 0.0 null null null)
  (`GameplayStatics.SpawnEmitterAtLocation` "/Game/StarterContent/Particles/P_Explosion.P_Explosion" HitLocation)
  (`self.K2_DestroyActor`))

(event `self.ReceiveDestroyed`
  ;[1 1 1] Dano no Jogador
  (`KismetSystemLibrary.PrintString` "BOOM!")
  (bind _asbp_game_mode (cast `/Game/Game/BP_GameMode` (`GameplayStatics.GetGameMode`)))
  (`/Game/Game/BP_GameMode.DanoJogador` _asbp_game_mode 10))

(fn `UserConstructionScript`)